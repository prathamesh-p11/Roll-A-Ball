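; Game mode that keeps the player's point count and shows a win message once the score reaches the goal.
; BeginPlay creates the BP_GameUI widget, adds it to the viewport and resets the score to zero.
; UpdatePoints increments the score, pushes it to the widget, then calls EndGame, which makes the win text visible at the threshold.
; A node that would hide the win text is left unconnected.
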(event Custom|ResetGame
  ;[1 1 1] Reset Game
  (Variables|Default|SetCurrentPoint 0)
  (Variables|/Game/Blueprints/BP_GameUI.BP_GameUI_C|SetPoint (Variables|Default|GetcurrentUI) 0))

(event Custom|UpdatePoints
  ;[1 1 1] Update Points
  (bind _output_get (Variables|Default|SetCurrentPoint (+ (Variables|Default|GetCurrentPoint) 1)))
  (Variables|/Game/Blueprints/BP_GameUI.BP_GameUI_C|SetPoint (Variables|Default|GetcurrentUI) _output_get)
  (CallFunction|EndGame))

(event Custom|End%20Game
  ;[1 1 1] Win Condition
  (if (>= (Variables|Default|GetCurrentPoint) 5)
    (Variables|/Game/Blueprints/BP_GameUI.BP_GameUI_C|SetyouWinOpacity (Variables|Default|GetcurrentUI) 1.0)))

(event EventBeginPlay
  ;[1 1 1] Create new UI instance and add to viewport
  (bind _returnvalue (UserInterface|CreateWidget "/Game/Blueprints/BP_GameUI.BP_GameUI_C"))
  (bind _output_get (Variables|Default|SetcurrentUI _returnvalue))
  (UserInterface|Viewport|AddtoViewport _output_get 0)
  (CallFunction|ResetGame))

(event EventTick
  (params (DeltaSeconds :type Float%20%28single-precision%29)))

(fn ConstructionScript)