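; BP_Coin_Pickup is a coin collectible that awards points when the player touches it.
; On overlap with BP_Player, it destroys itself and calls UpdatePoints on MyGameMode, which handles the scoring.
; Tick spins the Coin component by adding a speed set at BeginPlay to its relative roll each frame, without delta-time scaling.
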(event EventBeginPlay
  (Variables|Default|SetCoin_Rotation_Speed 1.5))

(event Collision|EventActorBeginOverlap
  (params (OtherActor :type Actor%20Object%20Reference))
  ;[1 1 1] If actor is overlapping, check if it is player, if it is, then destroy self
  (Utilities|Casting|CastToBP_Player OtherActor)
  (Actor|DestroyActor)
  (bind _asmy_game_mode (Utilities|Casting|CastToMyGameMode (Game|GetGameMode)))
  (Default|UpdatePoints _asmy_game_mode))

(event EventTick
  (params (DeltaSeconds :type Float%20%28single-precision%29))
  (bind _coin (Variables|Default|Getcoin))
  (bind _relativerotation (Variables|/Script/Engine.SceneComponent|GetRelativeRotation _coin))
  ;[1 1 1] Rotation animation
  (Transformation|SetRelativeRotation _coin (Math|Rotator|MakeRotator (+ (.roll _relativerotation) (Variables|Default|GetCoin_Rotation_Speed)) (.pitch _relativerotation) (.yaw _relativerotation)) false false))

(fn ConstructionScript)